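; BP_Enemy is an enemy that can be locked onto and absorbs fireballs.
; The Lockon event flip-flops the visibility of its Plane marker.
; Capsule overlap destroys any overlapping Fireball, with no damage applied to the enemy.
; DistanceToPlayer line-traces for pawns toward player 0 with debug drawing, stores the hit distance and sets CanBeTargeted to true regardless of the result.
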(event OnComponentBeginOverlap(CapsuleComponent)
  (params (OverlappedComponent :type Primitive%20Component%20Object%20Reference) (OtherActor :type Actor%20Object%20Reference) (OtherComp :type Primitive%20Component%20Object%20Reference) (OtherBodyIndex :type Integer) (bFromSweep :type Boolean) (SweepResult :type Hit%20Result%20Structure%20%28by%20ref%29))
  (bind _asfireball (Utilities|Casting|CastToFireball OtherActor))
  (Actor|DestroyActor _asfireball))

(event EventBeginPlay)

(event Collision|EventActorBeginOverlap
  (params (OtherActor :type Actor%20Object%20Reference)))

(event EventTick
  (params (DeltaSeconds :type Float%20%28single-precision%29)))

(event EventLockon
  (bind _plane (Variables|Default|GetPlane))
  (Utilities|FlowControl|FlipFlop
    (:A
      (Rendering|SetVisibility _plane true false))
    (:B
      (Rendering|SetVisibility _plane false false))))

(fn ConstructionScript)

(fn DistancetoPlayer
  (bind _outhit (Collision|LineTraceForObjects (Transformation|GetActorLocation) (Transformation|GetActorLocation (Game|Player|GetPlayerPawn 0)) (Utilities|Array|MakeArray "ObjectTypeQuery3") false (Utilities|Array|MakeArray self) "ForDuration" true "(R=1.000000,G=0.000000,B=0.000000,A=1.000000)" "(R=0.000000,G=1.000000,B=0.000000,A=1.000000)" 0.1))
  (Variables|Default|SetDistance (.Distance (Collision|BreakHitResult _outhit)))
  (Variables|Default|SetCan%20Be%20Targeted? true)
  (return))